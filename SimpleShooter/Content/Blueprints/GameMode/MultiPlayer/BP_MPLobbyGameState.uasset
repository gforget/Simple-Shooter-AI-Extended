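; Multiplayer lobby game state that tracks joined players, bots and the game type.
; Events add or remove players and bots, change teams or set the game type, writing each array back to its variable after edits.
; RepNotify functions for these variables find top-level WBP_Lobby widgets and call UpdateList with the current players, bots and game type.
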(event Custom|UpdateShooterPlayerStateTeam
  (params (PlayerId :type Integer) (Team :type ETeam%20Enum :default "BlueTeam"))
  (bind _returnvalue (Class|MPLobbyGameState|ReplaceTeaminPlayerState (Variables|Default|GetAllPlayerStates) PlayerId Team))
  (Variables|Default|SetAllPlayerStates _returnvalue))

(event Custom|PlayerJoined
  (params (JoinedPlayer :type Player%20State%20Object%20Reference))
  (bind _asshooter_player_state (Utilities|Casting|CastToShooterPlayerState JoinedPlayer))
  (Utilities|Array|Add (Variables|Default|GetAllPlayerStates) _asshooter_player_state)
  (Variables|Default|SetAllPlayerStates (Variables|Default|GetAllPlayerStates)))

(event Custom|PlayerLeft
  (params (Player%20Leaving :type Player%20State%20Object%20Reference))
  (bind _asshooter_player_state (Utilities|Casting|CastToShooterPlayerState Player%20Leaving))
  (Utilities|Array|RemoveItem (Variables|Default|GetAllPlayerStates) _asshooter_player_state)
  (Variables|Default|SetAllPlayerStates (Variables|Default|GetAllPlayerStates)))

(event Custom|RemoveBot
  (params (BotId :type Integer))
  (Utilities|Array|RemoveIndex (Variables|Default|GetAllBotsData) BotId)
  (Variables|Default|SetAllBotsData (Variables|Default|GetAllBotsData)))

(event Custom|AddBot
  (Utilities|Array|Add :TargetArray (Variables|Default|GetAllBotsData))
  (Variables|Default|SetAllBotsData (Variables|Default|GetAllBotsData)))

(event Custom|UpdateBotTeam
  (params (BotId :type Integer) (Team :type ETeam%20Enum :default "BlueTeam"))
  (bind _returnvalue (Class|MPLobbyGameState|ReplaceTeaminBotDatasArray (Variables|Default|GetAllBotsData) BotId Team))
  (Variables|Default|SetAllBotsData _returnvalue))

(event Custom|UpdateGameType
  (params (GameType :type EAllianceMode%20Enum :default "FFA"))
  (Variables|Default|SetGameType GameType))

(event EventBeginPlay)

(event EventTick
  (params (DeltaSeconds :type Float%20%28single-precision%29)))

(fn ConstructionScript)

(fn OnRepAllPlayerStates
  (bind _foundwidgets (Widget|GetAllWidgetsOfClass "/Game/Blueprints/UI/MultiplayerLobby/WBP_Lobby.WBP_Lobby_C" true))
  (for _array_element _foundwidgets
    (Default|UpdateList _array_element (Variables|Default|GetAllPlayerStates) (Variables|Default|GetAllBotsData) (Variables|Default|GetGameType))))

(fn OnRepAllBots
  (bind _foundwidgets (Widget|GetAllWidgetsOfClass "/Game/Blueprints/UI/MultiplayerLobby/WBP_Lobby.WBP_Lobby_C" true))
  (for _array_element _foundwidgets
    (Default|UpdateList _array_element (Variables|Default|GetAllPlayerStates) (Variables|Default|GetAllBotsData) (Variables|Default|GetGameType))))

(fn OnRepGameType
  (bind _foundwidgets (Widget|GetAllWidgetsOfClass "/Game/Blueprints/UI/MultiplayerLobby/WBP_Lobby.WBP_Lobby_C" true))
  (for _array_element _foundwidgets
    (Default|UpdateList _array_element (Variables|Default|GetAllPlayerStates) (Variables|Default|GetAllBotsData) (Variables|Default|GetGameType))))

(fn OnRepAllBotsData
  (bind _foundwidgets (Widget|GetAllWidgetsOfClass "/Game/Blueprints/UI/MultiplayerLobby/WBP_Lobby.WBP_Lobby_C" true))
  (for _array_element _foundwidgets
    (Default|UpdateList _array_element (Variables|Default|GetAllPlayerStates) (Variables|Default|GetAllBotsData) (Variables|Default|GetGameType))))